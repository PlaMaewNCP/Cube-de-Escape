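; BP_Key_Lv1 is a level 1 key pickup actor that the BP_CubeController actor collects by touching it.
; When its Box component overlaps an actor of exactly that class, it increments TotalLv1Key on BP_GameState.
; It then prints the new key total to the screen and destroys itself.
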(event `self.Box.OnComponentBeginOverlap`
  (params (OverlappedComponent :type "PrimitiveComponent Object Reference") (OtherActor :type "Actor Object Reference") (OtherComp :type "PrimitiveComponent Object Reference") (OtherBodyIndex :type Integer) (bFromSweep :type Boolean) (SweepResult :type "HitResult Structure (by ref)"))
  (if (== (`GameplayStatics.GetObjectClass` OtherActor) "/Game/Blueprints/BP_CubeController.BP_CubeController_C")
    (bind _asbp_game_state (cast `/Game/Blueprints/BP_GameState` (`GameplayStatics.GetGameState`)))
    (bind _output_get (set `/Game/Blueprints/BP_GameState.TotalLv1_Key` (+ (stale _output_get) 1) _asbp_game_state))
    (`KismetSystemLibrary.PrintString` (`KismetTextLibrary.Conv_TextToString` (`|FormatText` "Total Key log: {amount}" (`KismetStringLibrary.Conv_IntToString` _output_get))))
    (`self.K2_DestroyActor`)))

(event `self.ReceiveActorBeginOverlap`
  (params (OtherActor :type "Actor Object Reference")))

(fn `UserConstructionScript`)